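; BP_DamageNumber is a floating damage number actor that pops out with a random physics impulse.
; On BeginPlay it writes the truncated Damage value into its W_DamageNumber widget and tints the text by DamageType.
; A velocity-change impulse on the StaticMesh tosses it upward and sideways, and the actor destroys itself when the widget signals its lifetime is over.
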(event Custom|WidgetDead
  (Actor|DestroyActor))

(event EventBeginPlay
  (bind _asw_damage_number (Utilities|Casting|CastToW_DamageNumber (UserInterface|GetUserWidgetObject (Variables|Default|GetWidget))))
  (EventDispatchers|BindEventtoWidgetLifeTimeOver _asw_damage_number (delegate Custom|WidgetDead))
  (Rendering|Components|TextRender|SetText (Variables|/Game/DamageSystem/W_DamageNumber.W_DamageNumber_C|GetDamageValueText _asw_damage_number) (Utilities|Text|ToText(Integer) (Math|Float|Truncate (Variables|Default|GetDamage))))
  (Physics|AddImpulse (Variables|Default|GetStaticMesh) (Math|Vector|MakeVector (Math|Random|RandomFloatinRange -2e+02 2e+02) (Math|Random|RandomFloatinRange -2e+02 2e+02) (Math|Random|RandomFloatinRange 2e+02 4e+02)) "None" true)
  (switch Utilities|FlowControl|Switch|SwitchonE_DamageType (Variables|Default|GetDamageType)
    (:NewEnumerator1
      (Variables|Default|SetIn%20Color%20And%20Opacity%20Specified%20Color "(R=1.000000,G=1.000000,B=1.000000,A=1.000000)"))
    (:NewEnumerator2
      (Variables|Default|SetIn%20Color%20And%20Opacity%20Specified%20Color "(R=0.697917,G=0.218819,B=0.000000,A=1.000000)"))
    (:NewEnumerator3
      (Variables|Default|SetIn%20Color%20And%20Opacity%20Specified%20Color "(R=0.000000,G=0.619792,B=0.033124,A=1.000000)"))
    (:NewEnumerator5
      (Variables|Default|SetIn%20Color%20And%20Opacity%20Specified%20Color "(R=0.000000,G=0.446390,B=0.671875,A=1.000000)"))
    (:NewEnumerator6
      (bind _output_get (Variables|Default|SetIn%20Color%20And%20Opacity%20Specified%20Color "(R=0.442531,G=0.136719,B=0.729167,A=1.000000)"))))
  (Appearance|SetColorandOpacity (Variables|/Game/DamageSystem/W_DamageNumber.W_DamageNumber_C|GetDamageValueText _asw_damage_number) (Utilities|Struct|MakeSlateColor _output_get "UseColor_Specified") :!class /Script/UMG.TextBlock))

(fn ConstructionScript)