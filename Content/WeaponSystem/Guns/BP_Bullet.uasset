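; Projectile actor for the weapon system that damages whatever its sphere overlaps, then destroys itself.
; SetDamage supplies damage, type and special effects, and overlap sends them through the TakeDamage interface message.
; An explosive effect also spawns BP_Exsplosion at half damage.
; Tick yaw-billboards the FBBullet visual toward the camera.
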(event OnComponentBeginOverlap(Sphere)
  (params (OverlappedComponent :type Primitive%20Component%20Object%20Reference) (OtherActor :type Actor%20Object%20Reference) (OtherComp :type Primitive%20Component%20Object%20Reference) (OtherBodyIndex :type Integer) (bFromSweep :type Boolean) (SweepResult :type Hit%20Result%20Structure%20%28by%20ref%29))
  (Class|BPIDamageTable|TakeDamage(Message) OtherActor (Utilities|Struct|MakeS_DamageInfo (Variables|Default|GetDamge) "NewEnumerator1" (Variables|Default|GetDamage%20Type) false false))
  (for _array_element (Variables|Default|GetSpecialEffects)
    (switch Utilities|FlowControl|Switch|SwitchonE_SpecialEffects _array_element
      (:NewEnumerator1
        (Game|SpawnActorfromClass "/Game/Actors/BP_Exsplosion.BP_Exsplosion_C" (Math|Transform|MakeTransform (Transformation|GetActorLocation) "0, 0, 0" "2.000000,2.000000,2.000000") "Undefined" "MultiplyWithRoot" 0 (/ (Variables|Default|GetDamge) 2.0) (Variables|Default|GetDamage%20Type) 0))))
  (Actor|DestroyActor))

(event EventTick
  (params (DeltaSeconds :type Float%20%28single-precision%29))
  (bind _fb_bullet (Variables|Default|GetFB_Bullet))
  (Transformation|SetWorldRotation _fb_bullet (Math|Rotator|MakeRotator 0.0 -9e+01 (.yaw (Math|Rotator|MakeRotator 0.0 0.0 (+ (.Yaw (Math|Rotator|BreakRotator (Math|Rotator|FindLookatRotation (Transformation|GetWorldLocation _fb_bullet) (Camera|GetCameraLocation (Game|GetPlayerCameraManager 0))))) 9e+01)))) false false))

(event Collision|EventHit
  (params (MyComp :type Primitive%20Component%20Object%20Reference) (Other :type Actor%20Object%20Reference) (OtherComp :type Primitive%20Component%20Object%20Reference) (bSelfMoved :type Boolean) (HitLocation :type Vector :default "0, 0, 0") (HitNormal :type Vector :default "0, 0, 0") (NormalImpulse :type Vector :default "0, 0, 0") (Hit :type Hit%20Result%20Structure%20%28by%20ref%29))
  (Actor|DestroyActor))

(fn ConstructionScript)

(fn GetCurrentHealth
  (return 0.0))

(fn GetMaxHealth
  (return 0.0))

(fn Heal
  (params (Amount :type Float%20%28double-precision%29))
  (return 0.0))

(fn SetDamage
  (params (Damage :type Float%20%28double-precision%29) (DamageType :type E_DamageType%20Enum :default "NewEnumerator1") (SpecialEffects :type Array%20of%20E_SpecialEffects%20Enums :default "NewEnumerator0"))
  (Variables|Default|SetDamge Damage)
  (Variables|Default|SetDamage%20Type DamageType)
  (Variables|Default|SetSpecialEffects SpecialEffects)
  (return))

(fn TakeDamage
  (params (DamageInfo :type S%20Damage%20Info%20Structure))
  (return false))