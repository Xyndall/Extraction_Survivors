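; Master weapon Blueprint that handles firing, ammo, timed reloads (automatic when empty) and attachments.
; Stats live in the BPCGun component, seeded from WeaponItemInfo and scaled by attachments, which also add elemental damage types and special effects.
; Shoot spawns spread-randomized bullets, while LaserShoot line-traces and can spawn explosions, both picking a random damage type.
; A test widget displays current stats on screen.
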(event Custom|CheckSpecialEffects
  (bind _attachment (Variables|Default|GetAttachment))
  (if (.specialeffect _attachment)
    (switch Utilities|FlowControl|Switch|SwitchonE_SpecialEffects (.specialeffectenum _attachment)
      (:NewEnumerator0
        (Development|PrintString "No Effect"))
      (:NewEnumerator1
        (Utilities|Array|Add (Variables|Default|GetSpecialEffects) (.specialeffectenum _attachment) :!label _label))
      (:NewEnumerator2
        (goto _label))
      (:NewEnumerator3
        (goto _label)))
    (else
      (Development|PrintString "No Special Effect"))))

(event Custom|UpdateOscillation
  (bind (_newvalue _newdirection) (CallFunction|OscillatingFloat 0.0 (Variables|/Game/WeaponSystem/Guns/BPC_Gun.BPC_Gun_C|GetBulletSpread (Variables|Default|GetBPC_Gun)) 0.0)))

(event Custom|ReloadComplete
  ;[1 1 1] Reload
  (CallFunction|Reload)
  (Variables|Default|SetReloading? false))

(event EventRemoveAttachments
  (params (Attachment :type S%20Attachment%20Info%20Structure))
  (bind _damagetypes (Variables|Default|GetDamageTypes))
  (Utilities|Array|RemoveItem _damagetypes (.elementaldamage Attachment))
  (if (Utilities|Array|IsEmpty _damagetypes)
    (Utilities|Array|Add _damagetypes "NewEnumerator1")))

(event EventReloading
  ;[1 1 1] Reload
  (if (not (Variables|Default|GetReloading?))
    (Variables|Default|SetReloading? true)
    (bind _returnvalue (Utilities|Time|SetTimerbyEvent (delegate Custom|ReloadComplete) (Variables|/Game/WeaponSystem/Guns/BPC_Gun.BPC_Gun_C|GetReloadSpeed (Variables|Default|GetBPC_Gun))))
    (Variables|Default|SetReloadTimer _returnvalue)))

(event EventTick
  (params (DeltaSeconds :type Float%20%28single-precision%29))
  ;[1 1 1] AutoReload
  (if (and (<= (Variables|Default|GetCurrentAmmo) 0) (not (Variables|Default|GetReloading?)))
    (CallFunction|Reloading)))

(event EventBeginPlay
  (bind (_damage _firerate _magsize _spread _numofprojectiles _reloadspeed) (CallFunction|GunVariables))
  ;[1 1 1] Testing purposes. Shows gun stats on screen text widgets instead of printing stats.
  (Utilities|SetVariables
    (:Out
      (bind _returnvalue (UserInterface|CreateWidget "/Game/Character/W_PlayerStats.W_PlayerStats_C"))
      (UserInterface|Viewport|AddtoViewport _returnvalue 0)
      (Default|SetText _returnvalue (Utilities|Text|ToText(Float) _damage "HalfToEven") (Utilities|Text|ToText(Float) _firerate "HalfToEven") (Utilities|Text|ToText(Float) _spread "HalfToEven") (Utilities|Text|ToText(Integer) _magsize) (Utilities|Text|ToText(Integer) _numofprojectiles) (Utilities|Text|ToText(Float) _reloadspeed "HalfToEven")))))

(event EventGetProjectileSpawn
  (params (ProjectileSpawn :type Transform))
  (bind _output_get (Variables|Default|SetSpawnTransform ProjectileSpawn))
  (Transformation|SetWorldRotation (Variables|Default|GetArrow) (.rotation _output_get) false false))

(event EventAddAttachment
  (params (Attachment :type S%20Attachment%20Info%20Structure))
  (bind (_damage _firerate _magsize _spread _numofprojectiles _reloadspeed) (CallFunction|GunVariables))
  (bind (_damage_2 _firerate_2 _magsize_2 _spread_2 _numofprojectiles_2 _reloadspeed_2) (CallFunction|GunVariables))
  (bind _damagetypes (Variables|Default|GetDamageTypes))
  (bind _output_get (Variables|Default|SetAttachment Attachment))
  (Utilities|Array|Add _damagetypes (.elementaldamage _output_get))
  (for _array_element _damagetypes
    (if (Utilities|Enum|NotEqual(Enum) _array_element "NewEnumerator1")
      (Utilities|Array|RemoveItem (Variables|Default|GetDamageTypes) "NewEnumerator1")))
  (CallFunction|CheckSpecialEffects)
  (Default|UpdateVariables (Variables|Default|GetBPC_Gun) (Math|Conversions|ToFloat(Integer) (Math|Float|Round (+ _damage (* _damage (.damagemultipliers (Variables|Default|GetAttachment)))))) (+ _firerate (* _firerate (.rofmultipliers (Variables|Default|GetAttachment)))) (Math|Float|Round (+ _magsize (* _magsize (.magazinemultipliers (Variables|Default|GetAttachment))))) (+ _spread (* _spread (.bulletspreadmultipliers (Variables|Default|GetAttachment)))) (+ _numofprojectiles (.numberofprojectiles (Variables|Default|GetAttachment))) (+ _reloadspeed (* (* _reloadspeed (.reloadspeedmultipliers (Variables|Default|GetAttachment))) -1.0)))
  ;[1 1 1] updates text widgets to show new values after attachment is added
  (Default|SetText (stale EventBeginPlay _returnvalue) (Utilities|Text|ToText(Float) _damage_2 "HalfToEven") (Utilities|Text|ToText(Float) _firerate_2 "HalfToEven") (Utilities|Text|ToText(Float) _spread_2 "HalfToEven") (Utilities|Text|ToText(Integer) _magsize_2) (Utilities|Text|ToText(Integer) _numofprojectiles_2) (Utilities|Text|ToText(Float) _reloadspeed_2 "HalfToEven")))

(fn ConstructionScript)

(fn Shoot
  (bind (_damage _firerate _magsize _spread) (CallFunction|GunVariables))
  (bind _spawntransform (Variables|Default|GetSpawnTransform))
  (bind (_location _rotation) (Math|Transform|BreakTransform _spawntransform))
  ;[1 1 1] Spawns bullet at position
  (bind _returnvalue (Game|SpawnActorfromClass "/Game/WeaponSystem/Guns/BP_Bullet.BP_Bullet_C" (Math|Transform|MakeTransform _location (Math|Rotator|MakeRotator 0.0 0.0 (+ (.yaw _rotation) (Math|Random|RandomFloatinRange (* _spread -1.0) _spread))) "1.000000,1.000000,1.000000") "Undefined" "MultiplyWithRoot" 0 0))
  ;[1 1 1] Calculate damage in here
  (Class|BPIDamageTable|SetDamage(Message) _returnvalue _damage (.OutItem (Utilities|Array|Random (Variables|Default|GetDamageTypes))) (Variables|Default|GetSpecialEffects))
  ;[1 1 1] Camera shake
  (Class|LegacyCameraShake|StartLegacyCameraShake (Game|GetPlayerCameraManager 0) "/Game/Character/BP_CameraShake.BP_CameraShake_C" 1.0 "CameraLocal" "0, 0, 0"))

(fn UseAmmo
  (bind _output_get (Variables|Default|SetCurrentAmmo (Math|Integer|Clamp(Integer) (- (Variables|Default|GetCurrentAmmo) 1) 0 (Variables|/Game/WeaponSystem/Guns/BPC_Gun.BPC_Gun_C|GetMagSize (Variables|Default|GetBPC_Gun))))))

(fn Reload
  (Variables|Default|SetCurrentAmmo (.MagSize (CallFunction|GunVariables))))

(fn CheckCanFire
  (return (or (and (not (Variables|Default|GetReloading?)) (!= (Variables|Default|GetCurrentAmmo) 0)) (and (not (Variables|Default|GetReloading?)) (!= (Variables|Default|GetCurrentAmmo) -1)))))

(fn GunVariables
  (bind _bpc_gun (Variables|Default|GetBPC_Gun))
  (return (Variables|/Game/WeaponSystem/Guns/BPC_Gun.BPC_Gun_C|GetDamage _bpc_gun) (Variables|/Game/WeaponSystem/Guns/BPC_Gun.BPC_Gun_C|GetFireRate _bpc_gun) (Variables|/Game/WeaponSystem/Guns/BPC_Gun.BPC_Gun_C|GetMagSize _bpc_gun) (Variables|/Game/WeaponSystem/Guns/BPC_Gun.BPC_Gun_C|GetBulletSpread _bpc_gun) (Variables|/Game/WeaponSystem/Guns/BPC_Gun.BPC_Gun_C|GetNumOfProjectiles _bpc_gun) (Variables|/Game/WeaponSystem/Guns/BPC_Gun.BPC_Gun_C|GetReloadSpeed _bpc_gun)))

(fn LaserShoot
  (params (randomfloat :type Float%20%28double-precision%29))
  (bind _damage (CallFunction|GunVariables))
  (bind _damagetypes (Variables|Default|GetDamageTypes))
  (bind _arrow (Variables|Default|GetArrow))
  (bind _outitem (Utilities|Array|Random _damagetypes))
  (bind _returnvalue (Transformation|GetWorldLocation _arrow))
  ;[1 1 1] Spawns bullet at position
  (bind (_outhit _returnvalue_2) (Collision|LineTraceByChannel _returnvalue (+ _returnvalue (* (Math|Vector|GetForwardVector (Math|Rotator|MakeRotator 0.0 0.0 (+ (.Yaw (Math|Rotator|BreakRotator (Transformation|GetWorldRotation (Variables|Default|GetArrow)))) 0.0))) 2e+03)) "TraceTypeQuery4" true 0 "None"))
  (if _returnvalue_2
    ;[1 1 1] Calculate damage in here
    (Class|BPIDamageTable|TakeDamage(Message) (.HitActor (Collision|BreakHitResult _outhit)) (Utilities|Struct|MakeS_DamageInfo _damage "NewEnumerator0" _outitem false false))
    (for _array_element (Variables|Default|GetSpecialEffects)
      (switch Utilities|FlowControl|Switch|SwitchonE_SpecialEffects _array_element
        (:NewEnumerator1
          (Game|SpawnActorfromClass "/Game/Actors/BP_Exsplosion.BP_Exsplosion_C" (Math|Transform|MakeTransform (.Location (Collision|BreakHitResult _outhit)) "0, 0, 0" "2.000000,2.000000,2.000000") "Undefined" "MultiplyWithRoot" 0 (/ _damage 2.0) _outitem 0))))))

(fn CurrentAttachment
  (return 0))

(fn GetAmmoAmount
  (return (Variables|Default|GetCurrentAmmo) (Variables|/Game/WeaponSystem/Guns/BPC_Gun.BPC_Gun_C|GetMagSize (Variables|Default|GetBPC_Gun))))

(fn GetCurrentHealth
  (return 0.0))

(fn GetMaxHealth
  (return 0.0))

(fn GetReloadSpeed
  (return (Variables|/Game/WeaponSystem/Guns/BPC_Gun.BPC_Gun_C|GetReloadSpeed (Variables|Default|GetBPC_Gun))))

(fn GetReloadTimer
  (return (Variables|Default|GetReloadTimer) (Variables|Default|GetReloading?)))

(fn Heal
  (params (Amount :type Float%20%28double-precision%29))
  (return 0.0))

(fn ReturnItemInfo
  (params (WeaponItemInfo :type S%20Weapon%20Info%20Structure))
  (Variables|Default|SetWeapon%20Item%20Info WeaponItemInfo)
  (return))

(fn SetDamage
  (params (Damage :type Float%20%28double-precision%29) (DamageType :type E_DamageType%20Enum :default "NewEnumerator1") (SpecialEffects :type Array%20of%20E_SpecialEffects%20Enums :default "NewEnumerator0"))
  (return))

(fn TakeDamage
  (params (DamageInfo :type S%20Damage%20Info%20Structure))
  (return false))