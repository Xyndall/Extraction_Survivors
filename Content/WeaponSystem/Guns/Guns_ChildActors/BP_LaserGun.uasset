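; Laser gun weapon actor that loads its LaserGun row from DT_WeaponStats and fires automatically while the trigger is held.
; A gate and re-armed timer pace shots by FireRate, each calling LaserShoot per projectile with camera shake and consuming ammo.
; Each tick, LaserBeam drives a once-spawned Niagara beam, setting its end with a yaw-only line trace and zeroing particle counts when firing stops.
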(event Custom|AutoFire
  ;[0 0 0] FireRateLoop
  (Utilities|FlowControl|Gate true
    (:Exit
      (bind _returnvalue (Utilities|Time|SetTimerbyEvent (delegate Custom|AutoFire) (/ 1.0 (Variables|/Game/WeaponSystem/Guns/BPC_Gun.BPC_Gun_C|GetFireRate (Variables|Default|GetBPC_Gun)))))
      (bind _canfire (CallFunction|CheckCanFire))
      (if _canfire
        (for _index (range 1 (Variables|/Game/WeaponSystem/Guns/BPC_Gun.BPC_Gun_C|GetNumOfProjectiles (Variables|Default|GetBPC_Gun)))
          (Utilities|FlowControl|Sequence
            (:then_0
              (CallFunction|LaserShoot 0.0)
              ;;[1 1 1] Camera shake
              (Class|LegacyCameraShake|StartLegacyCameraShake (Game|GetPlayerCameraManager 0) "/Game/Character/BP_CameraShake.BP_CameraShake_C" 1.0 "CameraLocal" "0, 0, 0"))
            (:then_1
              (Utilities|FlowControl|DoOnce false
                (:Completed
                  (CallFunction|UseAmmo))))))
        (Utilities|FlowControl|DoOnce false) ; enters at Reset
      ))))

(event EventBeginPlay
  (|CallParentFunction))

(event Collision|EventActorBeginOverlap
  (params (OtherActor :type Actor%20Object%20Reference))
  (|CallParentFunction OtherActor) ; This node is disabled and will not be called.\nDrag off pins to build functionality.
)

(event EventFinishedFire
  (params (Fire :type Boolean))
  ;[0 0 0] FireRateLoop
  (Variables|Default|SetFire_0 false)
  (Utilities|FlowControl|Gate true) ; enters at Close
)

(event EventTick
  (params (DeltaSeconds :type Float%20%28single-precision%29))
  (|CallParentFunction DeltaSeconds)
  (Utilities|LaserBeam))

(event EventFire
  (params (Fire :type Boolean))
  ;[0 0 0] FireRateLoop
  (bind _canfire (CallFunction|CheckCanFire))
  (if _canfire
    (Variables|Default|SetFire_0 Fire)
    (Utilities|FlowControl|Sequence
      (:then_0
        (Utilities|FlowControl|Gate true) ; enters at Open
      )
      (:then_1
        (if (not (> (Utilities|Time|GetTimerRemainingTimebyHandle (stale _returnvalue)) 0.0))
          (bind _returnvalue (Utilities|Time|SetTimerbyEvent (delegate Custom|AutoFire) (/ 1.0 (Variables|/Game/WeaponSystem/Guns/BPC_Gun.BPC_Gun_C|GetFireRate (Variables|Default|GetBPC_Gun)))))
          (bind _canfire_2 (CallFunction|CheckCanFire))
          (if _canfire_2
            (for _index (range 1 (Variables|/Game/WeaponSystem/Guns/BPC_Gun.BPC_Gun_C|GetNumOfProjectiles (Variables|Default|GetBPC_Gun)))
              (Utilities|FlowControl|Sequence
                (:then_0
                  (CallFunction|LaserShoot 0.0)
                  ;;[1 1 1] Camera shake
                  (Class|LegacyCameraShake|StartLegacyCameraShake (Game|GetPlayerCameraManager 0) "/Game/Character/BP_CameraShake.BP_CameraShake_C" 1.0 "CameraLocal" "0, 0, 0"))
                (:then_1
                  (Utilities|FlowControl|DoOnce false
                    (:Completed
                      (CallFunction|UseAmmo))))))
            (Utilities|FlowControl|DoOnce false) ; enters at Reset
          ))))
    (else
      (Variables|Default|SetFire_0 false))))

(fn ConstructionScript
  (|CallParentFunction)
  (bind _returnvalue (Utilities|GetDataTableRow "/Game/WeaponSystem/Guns/Data/DT_WeaponStats.DT_WeaponStats" "LaserGun")
    (:then
      (Variables|Default|SetWeapon%20Item%20Info _returnvalue))))