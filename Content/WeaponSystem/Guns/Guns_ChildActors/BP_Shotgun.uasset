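; Shotgun weapon Blueprint that fires multiple projectiles per shot while consuming ammo once.
; Fire stores the spawn transform, checks whether it can fire, then calls the inherited Shoot once for each projectile in WeaponItemInfo.NumOfProjectiles.
; A DoOnce inside the loop limits UseAmmo to the first iteration and resets when the loop completes.
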(event EventBeginPlay
  (|CallParentFunction))

(event Collision|EventActorBeginOverlap
  (params (OtherActor :type Actor%20Object%20Reference))
  (|CallParentFunction OtherActor) ; This node is disabled and will not be called.\nDrag off pins to build functionality.
)

(event EventTick
  (params (DeltaSeconds :type Float%20%28single-precision%29))
  (|CallParentFunction DeltaSeconds) ; This node is disabled and will not be called.\nDrag off pins to build functionality.
)

(event EventFire
  (params (SpawnTransform :type Transform))
  (Variables|Default|SetSpawnTransform SpawnTransform)
  (bind _canfire (CallFunction|CheckCanFire))
  (if _canfire
    (for _index (range 1 (.numofprojectiles (Variables|Default|GetWeapon%20Item%20Info)))
      (Utilities|FlowControl|Sequence
        (:then_0
          (Utilities|FlowControl|DoOnce false
            (:Completed
              (CallFunction|UseAmmo))))
        (:then_1
          (CallFunction|Shoot))))
    (Utilities|FlowControl|DoOnce false) ; enters at Reset
  ))

(fn ConstructionScript
  (|CallParentFunction))