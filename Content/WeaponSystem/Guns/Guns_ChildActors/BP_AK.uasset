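; BP_AK is the AK rifle Blueprint in the weapon system, a gun child actor that builds on inherited firing logic.
; Fire stores the incoming spawn transform, then calls Shoot only if CheckCanFire passes.
; SetDamage returns the Damage value from WeaponItemInfo, while Tick and the construction script just call the parent.
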(event EventBeginPlay
  (|CallParentFunction) ; This node is disabled and will not be called.\nDrag off pins to build functionality.
)

(event Collision|EventActorBeginOverlap
  (params (OtherActor :type Actor%20Object%20Reference))
  (|CallParentFunction OtherActor) ; This node is disabled and will not be called.\nDrag off pins to build functionality.
)

(event EventTick
  (params (DeltaSeconds :type Float%20%28single-precision%29))
  (|CallParentFunction DeltaSeconds))

(event EventFire
  (params (SpawnTransform :type Transform))
  (Variables|Default|SetSpawnTransform SpawnTransform)
  (bind _canfire (CallFunction|CheckCanFire))
  (if _canfire
    (CallFunction|Shoot)))

(fn ConstructionScript
  (|CallParentFunction))

(fn SetDamage
  (params (Damage :type Float%20%28double-precision%29))
  (return (.damage (Variables|Default|GetWeapon%20Item%20Info))))