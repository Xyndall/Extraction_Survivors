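; BP_Bullet is a weapon-system bullet actor that damages whatever overlaps its Sphere collision.
; Each tick it billboards FBBullet toward the player camera on yaw only, with fixed pitch.
; On overlap it sends an interface TakeDamage message carrying the value stored by SetDamage, with no filtering or self-destruction.
; Its own health, heal and take-damage functions are stubs returning zero or false.
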(event OnComponentBeginOverlap(Sphere)
  (params (OverlappedComponent :type Primitive%20Component%20Object%20Reference) (OtherActor :type Actor%20Object%20Reference) (OtherComp :type Primitive%20Component%20Object%20Reference) (OtherBodyIndex :type Integer) (bFromSweep :type Boolean) (SweepResult :type Hit%20Result%20Structure%20%28by%20ref%29))
  (Class|BPIDamageTable|TakeDamage(Message) OtherActor (Utilities|Struct|MakeS_DamageInfo (Variables|Default|GetDamge) "NewEnumerator1" "NewEnumerator1" false false)))

(event EventTick
  (params (DeltaSeconds :type Float%20%28single-precision%29))
  (bind _fb_bullet (Variables|Default|GetFB_Bullet))
  (Transformation|SetWorldRotation _fb_bullet (Math|Rotator|MakeRotator 0.0 -9e+01 (.yaw (Math|Rotator|MakeRotator 0.0 0.0 (+ (.Yaw (Math|Rotator|BreakRotator (Math|Rotator|FindLookatRotation (Transformation|GetWorldLocation _fb_bullet) (Camera|GetCameraLocation (Game|GetPlayerCameraManager 0))))) 9e+01)))) false false))

(fn ConstructionScript)

(fn GetCurrentHealth
  (return 0.0))

(fn GetMaxHealth
  (return 0.0))

(fn Heal
  (params (Amount :type Float%20%28double-precision%29))
  (return 0.0))

(fn SetDamage
  (params (Damage :type Float%20%28double-precision%29))
  (bind _output_get (Variables|Default|SetDamge Damage))
  (return _output_get))

(fn TakeDamage
  (params (DamageInfo :type S%20Damage%20Info%20Structure))
  (return false))