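; BP_BugEnemy is a sprite-based enemy that chases the player and attacks on a looping timer.
; Tick drives AIMoveTo, faces the actor at the player, yaw-billboards the sprite to the camera and flips it by Y velocity.
; Attacks sphere-trace forward, sending damage and spawning particles on hit.
; BPCDamageSystem handles damage, healing and death through forwarded calls and bound events, with a health bar widget attached.
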(event Custom|Attack
  (bind _returnvalue (Transformation|GetActorLocation))
  (bind (_outhit _returnvalue_2) (Collision|SphereTraceForObjects _returnvalue (+ _returnvalue (* (Transformation|GetActorForwardVector) (Variables|Default|GetAttackRange))) 1e+02 (Utilities|Array|MakeArray "ObjectTypeQuery9") false 0 "ForDuration" true "(R=1.000000,G=0.000000,B=0.000000,A=1.000000)" "(R=0.000000,G=1.000000,B=0.000000,A=1.000000)" 1.0))
  (if _returnvalue_2
    (Class|BPIDamageTable|TakeDamage(Message) (.HitActor (Collision|BreakHitResult _outhit)) (Utilities|Struct|MakeS_DamageInfo 1e+01 "NewEnumerator1" "NewEnumerator1"))
    (if true
      (Effects|SpawnEmitteratLocation "/Engine/Tutorial/SubEditors/TutorialAssets/TutorialParticleSystem.TutorialParticleSystem" (.Location (Collision|BreakHitResult _outhit))))))

(event Custom|Death
  (Development|PrintString "Dead")
  (Actor|DestroyActor))

(event Custom|DamageResponse
  (params (DamageResponse :type E_DamageResponse%20Enum :default "NewEnumerator0"))
  (Development|PrintString (Utilities|String|EnumtoString DamageResponse)))

(event EventBeginPlay
  (Utilities|FlowControl|Sequence
    (:then_0
      ;[1 1 1] Begin play
      (bind _returnvalue (UserInterface|CreateWidget "/Game/DamageSystem/W_HealthBar.W_HealthBar_C" 0 self))
      (UserInterface|SetWidget (Variables|Default|GetHealthWidget) _returnvalue))
    (:then_1
      (Utilities|Time|SetTimerbyEvent (delegate Custom|Attack) 2.0 true))))

(event EventTick
  (params (DeltaSeconds :type Float%20%28single-precision%29))
  (bind _returnvalue (Game|GetPlayerCharacter 0))
  (bind _returnvalue_2 (Game|GetPlayerCameraManager 0))
  (bind _returnvalue_3 (Transformation|GetActorLocation))
  (bind _sprite (Variables|Default|GetSprite))
  (bind _sprite_2 (Variables|Default|GetSprite))
  (bind _returnvalue_4 (Transformation|GetWorldLocation _sprite_2))
  (bind _returnvalue_5 (Camera|GetCameraLocation _returnvalue_2))
  (bind _returnvalue_6 (Transformation|GetActorLocation _returnvalue))
  (bind _returnvalue_7 (Math|Rotator|FindLookatRotation _returnvalue_3 _returnvalue_6))
  (bind _returnvalue_8 (Math|Rotator|FindLookatRotation _returnvalue_4 _returnvalue_5))
  (bind _yaw (Math|Rotator|BreakRotator _returnvalue_8))
  (bind _returnvalue_9 (+ _yaw -9e+01))
  (bind _returnvalue_10 (Math|Rotator|MakeRotator 0.0 0.0 _returnvalue_9))
  ;[1 1 1] Tick
  (AI|AIMoveTo self "0, 0, 0" (Game|GetPlayerCharacter 0) 5.0 false
    (:then
      (Transformation|SetWorldRotation (Variables|Default|GetSprite) (Math|Rotator|MakeRotator (.roll _returnvalue_10) 0.0 (.yaw _returnvalue_10)) false false)
      (Transformation|SetActorRotation (Math|Rotator|MakeRotator (.roll _returnvalue_7) 0.0 (.yaw _returnvalue_7)))
      (if (> (.y (Transformation|GetVelocity)) 0.0)
        (Transformation|SetWorldScale3D _sprite (Math|Vector|MakeVector -1.0 1.0 1.0))
        (else
          (Transformation|SetWorldScale3D _sprite (Math|Vector|MakeVector 1.0 1.0 1.0)))))))

(fn ConstructionScript
  (bind _bpc_damagesystem (Variables|Default|GetBPC_DamageSystem))
  (EventDispatchers|BindEventtoOnDeath _bpc_damagesystem (EventDispatchers|CreateEvent :!event Custom|Death))
  (EventDispatchers|BindEventtoOnDamageResponse _bpc_damagesystem (EventDispatchers|CreateEvent :!event Custom|DamageResponse)))

(fn GetCurrentHealth
  (return (Variables|/Game/DamageSystem/BPC_DamageSystem.BPC_DamageSystem_C|GetHealth (Variables|Default|GetBPC_DamageSystem))))

(fn GetMaxHealth
  (return (Variables|/Game/DamageSystem/BPC_DamageSystem.BPC_DamageSystem_C|GetMaxHealth (Variables|Default|GetBPC_DamageSystem))))

(fn Heal
  (params (Amount :type Float%20%28double-precision%29))
  (bind _newhealth (Class|BPIDamageTable|Heal(Message) (Variables|Default|GetBPC_DamageSystem) Amount))
  (return _newhealth))

(fn SetDamage
  (params (Damage :type Float%20%28double-precision%29))
  (return 0.0))

(fn TakeDamage
  (params (DamageInfo :type S%20Damage%20Info%20Structure))
  (bind _wasdamaged (Default|TakeDamage (Variables|Default|GetBPC_DamageSystem) DamageInfo))
  (return _wasdamaged))