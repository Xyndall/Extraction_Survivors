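; Bug enemy with a health bar widget that attacks on a looping timer and awards XP to the player on death.
; Each attack sphere-traces forward, damaging the hit actor and spawning a particle effect.
; BPCDamageSystem handles health, healing, damage and death, with one damage type having a chance to start burning.
; Tick is empty, and the chase and sprite-billboarding logic is disconnected, so it never runs.
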(event Custom|DamageResponse
  (params (DamageResponse :type E_DamageResponse%20Enum :default "NewEnumerator0") (DamageType :type E_DamageType%20Enum :default "NewEnumerator1"))
  (if (Utilities|Enum|Equal(Enum) DamageType "NewEnumerator2")
    (bind _randomchance (CallFunction|DetermineChance 25.0))
    (Default|StartBurn (Variables|Default|GetBPC_DamageSystem) _randomchance)))

(event Custom|Death
  (Development|PrintString "Dead")
  (Class|BPITopDownChar|AddXP(Message) (Game|GetPlayerCharacter 0) (Variables|Default|GetXpDrop))
  (Actor|DestroyActor))

(event Custom|Attack
  (bind _returnvalue (Transformation|GetActorLocation))
  (bind (_outhit _returnvalue_2) (Collision|SphereTraceForObjects _returnvalue (+ _returnvalue (* (Transformation|GetActorForwardVector) (Variables|Default|GetAttackRange))) 1e+02 (Utilities|Array|MakeArray "ObjectTypeQuery9") false 0 "ForDuration" true "(R=1.000000,G=0.000000,B=0.000000,A=1.000000)" "(R=0.000000,G=1.000000,B=0.000000,A=1.000000)" 1.0))
  (if _returnvalue_2
    (Class|BPIDamageTable|TakeDamage(Message) (.HitActor (Collision|BreakHitResult _outhit)) (Utilities|Struct|MakeS_DamageInfo 1e+01 "NewEnumerator1"))
    (if true
      (Effects|SpawnEmitteratLocation "/Engine/Tutorial/SubEditors/TutorialAssets/TutorialParticleSystem.TutorialParticleSystem" (.Location (Collision|BreakHitResult _outhit))))))

(event EventBeginPlay
  (bind _bpc_damagesystem (Variables|Default|GetBPC_DamageSystem))
  (Utilities|FlowControl|Sequence
    (:then_0
      ;[1 1 1] Begin play
      (bind _returnvalue (UserInterface|CreateWidget "/Game/DamageSystem/W_HealthBar.W_HealthBar_C" 0 self))
      (UserInterface|SetWidget (Variables|Default|GetHealthWidget) _returnvalue)
      (bind _output_get (Variables|/Game/DamageSystem/BPC_DamageSystem.BPC_DamageSystem_C|SetMaxHealth _bpc_damagesystem 1e+04))
      (Variables|/Game/DamageSystem/BPC_DamageSystem.BPC_DamageSystem_C|SetHealth _bpc_damagesystem _output_get))
    (:then_1
      (Utilities|Time|SetTimerbyEvent (delegate Custom|Attack) 2.0 true))))

(event EventTick
  (params (DeltaSeconds :type Float%20%28single-precision%29))
  ;[1 1 1] Tick
)

(fn ConstructionScript
  (bind _bpc_damagesystem (Variables|Default|GetBPC_DamageSystem))
  (EventDispatchers|BindEventtoOnDeath _bpc_damagesystem (EventDispatchers|CreateEvent :!event Custom|Death))
  (EventDispatchers|BindEventtoOnDamageResponse _bpc_damagesystem (EventDispatchers|CreateEvent :!event Custom|DamageResponse)))

(fn GetCurrentHealth
  (return (Variables|/Game/DamageSystem/BPC_DamageSystem.BPC_DamageSystem_C|GetHealth (Variables|Default|GetBPC_DamageSystem))))

(fn GetMaxHealth
  (return (Variables|/Game/DamageSystem/BPC_DamageSystem.BPC_DamageSystem_C|GetMaxHealth (Variables|Default|GetBPC_DamageSystem))))

(fn GetXPandLevel
  (return 0.0 0.0 0))

(fn Heal
  (params (Amount :type Float%20%28double-precision%29))
  (bind _newhealth (Class|BPIDamageTable|Heal(Message) (Variables|Default|GetBPC_DamageSystem) Amount))
  (return _newhealth))

(fn SetDamage
  (params (Damage :type Float%20%28double-precision%29) (DamageType :type E_DamageType%20Enum :default "NewEnumerator1") (SpecialEffects :type Array%20of%20E_SpecialEffects%20Enums :default "NewEnumerator0"))
  (return))

(fn TakeDamage
  (params (DamageInfo :type S%20Damage%20Info%20Structure))
  (bind _wasdamaged (Default|TakeDamage (Variables|Default|GetBPC_DamageSystem) DamageInfo))
  (return _wasdamaged))