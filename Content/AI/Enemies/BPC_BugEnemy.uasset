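; Basic bug enemy Blueprint that supplies data-driven stats and a sphere-trace attack.
; Construction script loads the BasicBug row from DT_EnemyData into EnemyInfo.
; Attack sphere-traces with debug drawing from itself to the player-to-self unit direction scaled by AttackRange, without adding the actor's location.
; A hit sends damage amount and type from EnemyInfo to the hit actor, then returns the attack speed.
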(event EventBeginPlay
  (|CallParentFunction) ; This node is disabled and will not be called.\nDrag off pins to build functionality.
)

(event Collision|EventActorBeginOverlap
  (params (OtherActor :type Actor%20Object%20Reference)))

(event EventTick
  (params (DeltaSeconds :type Float%20%28single-precision%29))
  (|CallParentFunction DeltaSeconds) ; This node is disabled and will not be called.\nDrag off pins to build functionality.
)

(fn ConstructionScript
  (|CallParentFunction)
  (bind _returnvalue (Utilities|GetDataTableRow "/Game/AI/Data/DT_EnemyData.DT_EnemyData" "BasicBug")
    (:then
      (Variables|Default|SetEnemyInfo _returnvalue))))

(fn Attack
  (bind _enemyinfo (Variables|Default|GetEnemyInfo))
  (bind (_outhit _returnvalue) (Collision|SphereTraceForObjects (Transformation|GetActorLocation) (* (Math|Vector|GetUnitDirection(Vector) (Transformation|GetActorLocation (Game|GetPlayerCharacter 0)) (Transformation|GetActorLocation)) (Variables|Default|GetAttackRange)) 1e+02 (Utilities|Array|MakeArray "ObjectTypeQuery9") false 0 "ForDuration" true "(R=1.000000,G=0.000000,B=0.000000,A=1.000000)" "(R=0.000000,G=1.000000,B=0.000000,A=1.000000)" 1.0))
  (if _returnvalue
    (Class|BPIDamageTable|TakeDamage(Message) (.HitActor (Collision|BreakHitResult _outhit)) (Utilities|Struct|MakeS_DamageInfo (.damage _enemyinfo) "NewEnumerator1" (.damagetype _enemyinfo)))
    (return (.attackspped _enemyinfo))))