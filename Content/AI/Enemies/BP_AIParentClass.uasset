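; Parent class for enemy AI characters that chase the player with a camera-facing 2D sprite, flipped by velocity.
; EnemyInfo sets health, hit-sphere radius, damage and a looping attack timer.
; While the player overlaps the sphere, the timer fires a melee sphere trace or spawns a projectile.
; BPCDamageSystem handles damage, healing and death, which awards XP and destroys the enemy; one damage type can trigger burning.
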(event OnComponentBeginOverlap(HitRangeSphere)
  (params (OverlappedComponent :type Primitive%20Component%20Object%20Reference) (OtherActor :type Actor%20Object%20Reference) (OtherComp :type Primitive%20Component%20Object%20Reference) (OtherBodyIndex :type Integer) (bFromSweep :type Boolean) (SweepResult :type Hit%20Result%20Structure%20%28by%20ref%29))
  (if (Actor|ActorHasTag OtherActor "Player")
    (Variables|Default|SetPlayerInRange true)))

(event OnComponentEndOverlap(HitRangeSphere)
  (params (OverlappedComponent :type Primitive%20Component%20Object%20Reference) (OtherActor :type Actor%20Object%20Reference) (OtherComp :type Primitive%20Component%20Object%20Reference) (OtherBodyIndex :type Integer))
  (if (Actor|ActorHasTag OtherActor "Player")
    (Variables|Default|SetPlayerInRange false)))

(event Custom|Attack
  (Variables|Default|SetCanAttack false)
  (if (.isranged (Variables|Default|GetEnemyInfo))
    (CallFunction|RangedAttack)
    (else
      (CallFunction|MeleeAttack))))

(event Custom|DamageResponse
  (params (DamageResponse :type E_DamageResponse%20Enum :default "NewEnumerator0") (DamageType :type E_DamageType%20Enum :default "NewEnumerator1"))
  (if (Utilities|Enum|Equal(Enum) DamageType "NewEnumerator2")
    (bind _randomchance (CallFunction|DetermineChance 25.0))
    (Default|StartBurn (Variables|Default|GetBPC_DamageSystem) _randomchance)))

(event Custom|Death
  (Class|BPITopDownChar|AddXP(Message) (Game|GetPlayerCharacter 0) (.xpamount (Variables|Default|GetEnemyInfo)))
  (Actor|DestroyActor))

(event EventBeginPlay
  (Utilities|SetDataVariables
    (:Out
      (Utilities|FlowControl|Sequence
        (:then_0
          ;[1 1 1] Begin play
          (bind _returnvalue (UserInterface|CreateWidget "/Game/DamageSystem/W_HealthBar.W_HealthBar_C" 0 self))
          (UserInterface|SetWidget (Variables|Default|GetHealthWidget) _returnvalue))
        (:then_1
          (bind _returnvalue_2 (Utilities|Time|SetTimerbyFunctionName 0 "SetAttack" (.attackspped (Variables|Default|GetEnemyInfo)) true))
          (Variables|Default|SetPassiveAttackTimer _returnvalue_2))))))

(event EventTick
  (params (DeltaSeconds :type Float%20%28single-precision%29))
  (bind _returnvalue (Game|GetPlayerCameraManager 0))
  (bind _returnvalue_2 (Transformation|GetActorLocation))
  (bind _returnvalue_3 (Game|GetPlayerController 0))
  (bind _sprite (Variables|Default|GetSprite))
  (bind _sprite_2 (Variables|Default|GetSprite))
  (bind _returnvalue_4 (Transformation|GetActorLocation _returnvalue_3))
  (bind _returnvalue_5 (Transformation|GetWorldLocation _sprite_2))
  (bind _returnvalue_6 (Camera|GetCameraLocation _returnvalue))
  (bind _returnvalue_7 (Math|Rotator|FindLookatRotation _returnvalue_2 _returnvalue_4))
  (bind _returnvalue_8 (Math|Rotator|FindLookatRotation _returnvalue_5 _returnvalue_6))
  (bind _yaw (Math|Rotator|BreakRotator _returnvalue_8))
  (bind _returnvalue_9 (+ _yaw -9e+01))
  (bind _returnvalue_10 (Math|Rotator|MakeRotator 0.0 0.0 _returnvalue_9))
  (AI|AIMoveTo self "0, 0, 0" (Game|GetPlayerCharacter 0) 5.0 false
    (:then
      ;[1 1 1] calculates the rotation and which way the sprite should be flipped. if player is on left or right side of enemy sprite flips accordingly.
      (Transformation|SetWorldRotation (Variables|Default|GetSprite) (Math|Rotator|MakeRotator (.roll _returnvalue_10) 0.0 (.yaw _returnvalue_10)) false false)
      (Transformation|SetActorRotation self (Math|Rotator|MakeRotator (.roll _returnvalue_7) 0.0 (.yaw _returnvalue_7)))
      (if (> (.y (Transformation|GetVelocity)) 0.0)
        (Transformation|SetWorldScale3D _sprite (Math|Vector|MakeVector -1.0 1.0 1.0))
        (else
          (Transformation|SetWorldScale3D _sprite (Math|Vector|MakeVector 1.0 1.0 1.0)))))))

(fn ConstructionScript
  (bind _bpc_damagesystem (Variables|Default|GetBPC_DamageSystem))
  (EventDispatchers|BindEventtoOnDeath _bpc_damagesystem (EventDispatchers|CreateEvent :!event Custom|Death))
  (EventDispatchers|BindEventtoOnDamageResponse _bpc_damagesystem (EventDispatchers|CreateEvent :!event Custom|DamageResponse)))

(fn MeleeAttack
  (bind _returnvalue (Transformation|GetActorLocation))
  (bind _enemyinfo (Variables|Default|GetEnemyInfo))
  (bind (_outhit _returnvalue_2) (Collision|SphereTraceForObjects _returnvalue (+ _returnvalue (* (Transformation|GetActorForwardVector) (Variables|Default|GetAttackRange))) 1e+02 (Utilities|Array|MakeArray "ObjectTypeQuery9") true 0 "ForDuration" true "(R=1.000000,G=0.000000,B=0.000000,A=1.000000)" "(R=0.000000,G=1.000000,B=0.000000,A=1.000000)" 1.0))
  (if _returnvalue_2
    (Class|BPIDamageTable|TakeDamage(Message) (.HitActor (Collision|BreakHitResult _outhit)) (Utilities|Struct|MakeS_DamageInfo (.damage _enemyinfo) "NewEnumerator1" (.damagetype _enemyinfo)))
    (if true
      (Effects|SpawnEmitteratLocation "/Engine/Tutorial/SubEditors/TutorialAssets/TutorialParticleSystem.TutorialParticleSystem" (.Location (Collision|BreakHitResult _outhit))))))

(fn RangedAttack
  (bind _enemyinfo (Variables|Default|GetEnemyInfo))
  (bind _returnvalue (Game|SpawnActorfromClass "/Game/AI/Extra/BP_EnemyProjectile.BP_EnemyProjectile_C" (Math|Transform|MakeTransform (Transformation|GetActorLocation) (Math|Rotator|MakeRotator 0.0 0.0 (.yaw (Math|Conversions|RotationFromXVector (- (Transformation|GetActorLocation (Game|GetPlayerCharacter 0)) (Transformation|GetActorLocation))))) "1.000000,1.000000,1.000000") "Undefined" "MultiplyWithRoot" 0 0))
  (Default|SetDamage _returnvalue (.damage _enemyinfo) (.damagetype _enemyinfo) "NewEnumerator0"))

(fn SetAttack
  (if (Variables|Default|GetPlayerInRange)
    (CallFunction|Attack)))

(fn GetCurrentHealth
  (return (Variables|/Game/DamageSystem/BPC_DamageSystem.BPC_DamageSystem_C|GetHealth (Variables|Default|GetBPC_DamageSystem))))

(fn GetMaxHealth
  (return (Variables|/Game/DamageSystem/BPC_DamageSystem.BPC_DamageSystem_C|GetMaxHealth (Variables|Default|GetBPC_DamageSystem))))

(fn GetXPandLevel
  (return 0.0 0.0 0))

(fn Heal
  (params (Amount :type Float%20%28double-precision%29))
  (bind _newhealth (Class|BPIDamageTable|Heal(Message) (Variables|Default|GetBPC_DamageSystem) Amount))
  (return _newhealth))

(fn SetDamage
  (params (Damage :type Float%20%28double-precision%29) (DamageType :type E_DamageType%20Enum :default "NewEnumerator1") (SpecialEffects :type Array%20of%20E_SpecialEffects%20Enums :default "NewEnumerator0"))
  (return))

(fn TakeDamage
  (params (DamageInfo :type S%20Damage%20Info%20Structure))
  (bind _wasdamaged (Default|TakeDamage (Variables|Default|GetBPC_DamageSystem) DamageInfo))
  (return _wasdamaged))