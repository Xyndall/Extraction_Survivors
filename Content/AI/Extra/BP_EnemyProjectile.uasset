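; Enemy projectile that deals damage to overlapping actors and destroys itself on hit.
; Each tick, its Paper2D flipbook turns to face the player camera on yaw only, as a billboard sprite.
; Sphere overlap sends a damage message using the Damage and DamageType stored by SetDamage, which ignores SpecialEffects.
; Health, heal and take-damage functions are stubs returning zero or false.
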(event OnComponentBeginOverlap(Sphere)
  (params (OverlappedComponent :type Primitive%20Component%20Object%20Reference) (OtherActor :type Actor%20Object%20Reference) (OtherComp :type Primitive%20Component%20Object%20Reference) (OtherBodyIndex :type Integer) (bFromSweep :type Boolean) (SweepResult :type Hit%20Result%20Structure%20%28by%20ref%29))
  (Class|BPIDamageTable|TakeDamage(Message) OtherActor (Utilities|Struct|MakeS_DamageInfo (Variables|Default|GetDamage) "NewEnumerator1" (Variables|Default|GetDamageType) false false)))

(event EventTick
  (params (DeltaSeconds :type Float%20%28single-precision%29))
  (bind _paperflipbook (Variables|Default|GetPaperFlipbook))
  (Transformation|SetWorldRotation _paperflipbook (Math|Rotator|MakeRotator 0.0 -9e+01 (.yaw (Math|Rotator|MakeRotator 0.0 0.0 (+ (.Yaw (Math|Rotator|BreakRotator (Math|Rotator|FindLookatRotation (Transformation|GetWorldLocation _paperflipbook) (Camera|GetCameraLocation (Game|GetPlayerCameraManager 0))))) 9e+01)))) false false))

(event Collision|EventHit
  (params (MyComp :type Primitive%20Component%20Object%20Reference) (Other :type Actor%20Object%20Reference) (OtherComp :type Primitive%20Component%20Object%20Reference) (bSelfMoved :type Boolean) (HitLocation :type Vector :default "0, 0, 0") (HitNormal :type Vector :default "0, 0, 0") (NormalImpulse :type Vector :default "0, 0, 0") (Hit :type Hit%20Result%20Structure%20%28by%20ref%29))
  (Actor|DestroyActor))

(fn ConstructionScript)

(fn GetCurrentHealth
  (return 0.0))

(fn GetMaxHealth
  (return 0.0))

(fn Heal
  (params (Amount :type Float%20%28double-precision%29))
  (return 0.0))

(fn SetDamage
  (params (Damage :type Float%20%28double-precision%29) (DamageType :type E_DamageType%20Enum :default "NewEnumerator1") (SpecialEffects :type Array%20of%20E_SpecialEffects%20Enums :default "NewEnumerator0"))
  (Variables|Default|SetDamage Damage)
  (Variables|Default|SetDamageType DamageType)
  (return))

(fn TakeDamage
  (params (DamageInfo :type S%20Damage%20Info%20Structure))
  (return false))