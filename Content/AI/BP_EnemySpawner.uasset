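; Enemy spawner that periodically spawns random-sized batches of BPC_SpitterBug around the player and tracks them in EnemyArray.
; A looping timer, its random interval rolled once at BeginPlay, calls SpawnEnemy, which rerolls reachable nav points around the player controller until outside a minimum distance.
; IncreaseDifficulty raises SpawnCount and lowers the interval bounds without resetting the timer.
; NewWave removes array entries while iterating, without destroying actors.
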(event Custom|NewWave
  (bind _enemy_array (Variables|Default|GetEnemy%20Array))
  (for _array_element (Variables|Default|GetEnemy%20Array)
    (Utilities|IsValid _array_element
      (:Is%20Valid
        (Utilities|Array|RemoveItem _enemy_array _array_element))
      (:Is%20Not%20Valid
        (Utilities|Array|RemoveItem _enemy_array _array_element)))))

(event Custom|SpawnEnemy
  ;[1 1 1] Basic Spawner, Will Spawn Enemy by the second, Still need to find a better implementation
  (for _index (range 0 (Math|Random|RandomIntegerinRange 0 (Variables|Default|GetSpawnCount)))
    (bind _location (CallFunction|FindGoodLocation))
    (bind _returnvalue (Game|SpawnActorfromClass "/Game/AI/Enemies/BPC_SpitterBug.BPC_SpitterBug_C" (Math|Transform|MakeTransform _location "0, 0, 0" "1.000000,1.000000,1.000000") "Undefined" "MultiplyWithRoot" 0 0))
    (Utilities|Array|Add (Variables|Default|GetEnemy%20Array) _returnvalue)))

(event Custom|IncreaseDifficulty
  ;[1 1 1] Basic Spawner, Will Spawn Enemy by the second, Still need to find a better implementation
  (Math|Integer|IncrementInt (Variables|Default|GetSpawnCount)
    (:%20%20
      (Variables|Default|SetMin (Math|Float|Clamp(Float) (- (Variables|Default|GetMin) 0.2) 0.2 5.0))
      (Variables|Default|SetMax (Math|Float|Clamp(Float) (- (Variables|Default|GetMax) 0.2) 0.5 1e+01)))))

(event EventBeginPlay
  ;[1 1 1] Basic Spawner, Will Spawn Enemy by the second, Still need to find a better implementation
  (Utilities|Time|SetTimerbyEvent (delegate Custom|SpawnEnemy) (Math|Random|RandomFloatinRange (Variables|Default|GetMin) (Variables|Default|GetMax)) true))

(fn ConstructionScript)

(fn FindGoodLocation
  (bind _returnvalue (Game|GetPlayerController 0))
  (bind _returnvalue_2 (Transformation|GetActorLocation _returnvalue))
  (bind _randomlocation (AI|Navigation|GetRandomReachablePointinRadius _returnvalue_2 5e+03 0 0))
  (Variables|Default|SetRandomLocation _randomlocation)
  (while (< (Math|Vector|Distance(Vector) _returnvalue_2 (Variables|Default|GetRandomLocation)) 1.5e+03)
    (Variables|Default|SetRandomLocation _randomlocation))
  (return (Variables|Default|GetRandomLocation)))