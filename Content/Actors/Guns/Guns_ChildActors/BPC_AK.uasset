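; BPC_AK is the AK weapon child Blueprint, which supplies the gun's firing behavior.
; Its Fire event spawns a BP_Bullet at the given transform's location, adding a random yaw offset between the weapon item info's minimum and maximum spread.
; Tick and the construction script only call the parent.
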(event EventBeginPlay
  (|CallParentFunction) ; This node is disabled and will not be called.\nDrag off pins to build functionality.
)

(event Collision|EventActorBeginOverlap
  (params (OtherActor :type Actor%20Object%20Reference))
  (|CallParentFunction OtherActor) ; This node is disabled and will not be called.\nDrag off pins to build functionality.
)

(event EventTick
  (params (DeltaSeconds :type Float%20%28single-precision%29))
  (|CallParentFunction DeltaSeconds))

(event EventFire
  (params (SpawnTransform :type Transform))
  (bind (_location _rotation) (Math|Transform|BreakTransform SpawnTransform))
  (bind _weapon_item_info (Variables|Default|GetWeapon%20Item%20Info))
  (Game|SpawnActorfromClass "/Game/Actors/BP_Bullet.BP_Bullet_C" (Math|Transform|MakeTransform _location (Math|Rotator|MakeRotator 0.0 0.0 (+ (.yaw _rotation) (Math|Random|RandomFloatinRange (.minspread _weapon_item_info) (.maxspread _weapon_item_info)))) "1.000000,1.000000,1.000000") "Undefined" "MultiplyWithRoot" 0 0))

(fn ConstructionScript
  (|CallParentFunction))