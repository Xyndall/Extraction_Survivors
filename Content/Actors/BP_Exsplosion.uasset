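; Short-lived explosion actor that damages actors overlapping its sphere.
; On BeginPlay it spawns the explosion particle emitter at its location, scaled to the sphere, then destroys both emitter and itself after a brief delay.
; Sphere overlaps during that window send a TakeDamage message to the other actor, carrying the damage amount, type and a fixed response.
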(event OnComponentBeginOverlap(Sphere1)
  (params (OverlappedComponent :type Primitive%20Component%20Object%20Reference) (OtherActor :type Actor%20Object%20Reference) (OtherComp :type Primitive%20Component%20Object%20Reference) (OtherBodyIndex :type Integer) (bFromSweep :type Boolean) (SweepResult :type Hit%20Result%20Structure%20%28by%20ref%29))
  (Class|BPIDamageTable|TakeDamage(Message) OtherActor (Utilities|Struct|MakeS_DamageInfo (Variables|Default|GetDamageAmount) "NewEnumerator1" (Variables|Default|GetDamageType) false false)))

(event EventBeginPlay
  (bind _returnvalue (Effects|SpawnEmitteratLocation "/Game/Actors/Explosion.Explosion" (Transformation|GetActorLocation) "0, 0, 0" (Transformation|GetWorldScale (Variables|Default|GetSphere1))))
  (Utilities|FlowControl|Delay 0.3)
  (Components|DestroyComponent _returnvalue)
  (Actor|DestroyActor))

(fn ConstructionScript)