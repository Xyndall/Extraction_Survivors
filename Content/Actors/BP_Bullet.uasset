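; BP_Bullet is a projectile actor that passes damage to actors overlapping its sphere.
; Each tick it billboards the FBBullet component by yawing it toward the player camera with pitch and roll fixed.
; Sphere overlap sends the Damge value through a CalculateDamage interface message.
; Its own CalculateDamage is empty, and the actor overlap check for the PlayerProjectile tag leads to no action.
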(event OnComponentBeginOverlap(Sphere)
  (params (OverlappedComponent :type Primitive%20Component%20Object%20Reference) (OtherActor :type Actor%20Object%20Reference) (OtherComp :type Primitive%20Component%20Object%20Reference) (OtherBodyIndex :type Integer) (bFromSweep :type Boolean) (SweepResult :type Hit%20Result%20Structure%20%28by%20ref%29))
  (Class|BPIEnemy|CalculateDamage(Message) OtherActor (Variables|Default|GetDamge)))

(event EventBeginPlay)

(event EventTick
  (params (DeltaSeconds :type Float%20%28single-precision%29))
  (bind _fb_bullet (Variables|Default|GetFB_Bullet))
  (Transformation|SetWorldRotation _fb_bullet (Math|Rotator|MakeRotator 0.0 -9e+01 (.yaw (Math|Rotator|MakeRotator 0.0 0.0 (+ (.Yaw (Math|Rotator|BreakRotator (Math|Rotator|FindLookatRotation (Transformation|GetWorldLocation _fb_bullet) (Camera|GetCameraLocation (Game|GetPlayerCameraManager 0))))) 9e+01)))) false false))

(event Collision|EventActorBeginOverlap
  (params (OtherActor :type Actor%20Object%20Reference))
  (if (Actor|ActorHasTag OtherActor "PlayerProjectile")
    _))

(fn ConstructionScript)

(fn CalculateDamage
  (params (DamageIn :type Float%20%28double-precision%29)))