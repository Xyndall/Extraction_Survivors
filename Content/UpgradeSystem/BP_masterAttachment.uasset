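; Base pickup actor for weapon or upgrade attachments, named as the master class in the upgrade system.
; SetAttachment looks up a row in DT_AttachmentStats, stores it as AttachmentInfo and shows its icon on a Paper sprite.
; On overlap it passes that info to the other actor through an AddAttachmentMessage interface call, then destroys itself.
; AddAttachment, CurrentAttachment and RemoveAttachment are empty stubs here.
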(event EventBeginPlay)

(event Collision|EventActorBeginOverlap
  (params (OtherActor :type Actor%20Object%20Reference))
  (Class|BPIAttachments|AddAttachment(Message) OtherActor (Variables|Default|GetAttachmentInfo))
  (Actor|DestroyActor))

(fn ConstructionScript)

(fn SetAttachment
  (params (AttachmentName :type Name))
  (bind _returnvalue (Utilities|GetDataTableRow "/Game/UpgradeSystem/DT_AttachmentStats.DT_AttachmentStats" AttachmentName)
    (:then
      (bind _output_get (Variables|Default|SetAttachmentInfo _returnvalue))
      (Rendering|Components|Sprite|SetSprite (Variables|Default|GetPaperSprite) (.SpriteIcon (Utilities|Struct|BreakS_AttachmentInfo _output_get)))
      (return))
    (:RowNotFound
      (Development|PrintString "could not find"))))

(fn AddAttachment
  (params (Attachment :type S%20Attachment%20Info%20Structure))
  (return))

(fn CurrentAttachment
  (return 0))

(fn RemoveAttachment
  (return ""))