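; Upgrade system component that handles XP leveling and attachment stat lookups.
; AddXp accumulates XP and records the previous level, then on reaching the threshold raises the level once, carries over excess XP and increases MaxXP by a fixed step.
; On level-up it returns whether leftover XP still meets the new threshold.
; GetAttachment fetches a named row from DT_AttachmentStats, printing whether it was found.
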(event EventBeginPlay)

(event EventTick
  (params (DeltaSeconds :type Float%20%28single-precision%29)))

(fn GetAttachment
  (params (AttachmentName :type Name))
  (bind _returnvalue (Utilities|GetDataTableRow "/Game/UpgradeSystem/DT_AttachmentStats.DT_AttachmentStats" AttachmentName)
    (:then
      (bind _output_get (Variables|Default|SetAttachmentInfo _returnvalue))
      (Development|PrintText (Utilities|Text|FormatText "{Found attachment info} {attachment name}" 0 AttachmentName))
      (return _output_get))
    (:RowNotFound
      (Development|PrintString "Did not find attachment info"))))

(fn AddXp
  (params (xpAmount :type Float%20%28double-precision%29))
  (Variables|Default|SetXP (+ (Variables|Default|GetXP) xpAmount))
  (Variables|Default|SetLastLevel (Variables|Default|GetLevel))
  (if (>= (Variables|Default|GetXP) (Variables|Default|GetMaxXP))
    (Math|Integer|IncrementInt (Variables|Default|GetLevel)
      (:%20%20
        (Variables|Default|SetXP (- (Variables|Default|GetXP) (Variables|Default|GetMaxXP)))
        (Variables|Default|SetMaxXp (+ (Variables|Default|GetMaxXp) 2e+01))
        (return (>= (Variables|Default|GetXP) (Variables|Default|GetMaxXP)))))))